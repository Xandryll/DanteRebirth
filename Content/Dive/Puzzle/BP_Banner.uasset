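; BP_Banner is a rotatable ray puzzle piece that acts as emitter, blocker or relay, shown by green, red or blue material.
; Mouse use steps it through preset yaw angles.
; Emitters line-trace forward every second, activating any BPI_Dante actor hit, so non-emitters trace onward in a chain that blockers stop.
; Successful links appear as stacked green debug lines lasting one second.
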(event Custom|SendRay
  (bind _arrow (Variables|Default|GetArrow))
  (bind _returnvalue (Transformation|GetWorldLocation _arrow))
  (bind _outhit (Collision|LineTraceByChannel _returnvalue (+ _returnvalue (* (Math|Vector|GetForwardVector _arrow) 3e+04)) "TraceTypeQuery1" false 0 "None" true "(R=0.000000,G=0.954989,B=1.000000,A=1.000000)" "(R=1.000000,G=0.000000,B=0.972589,A=1.000000)" 1.0))
  (if (Utilities|DoesObjectImplementInterface (.HitActor (Collision|BreakHitResult _outhit)) "/Game/Dive/Puzzle/BPI_Dante.BPI_Dante_C")
    (if (not (Variables|Default|GetBlocker))
      (Class|BPIDante|ActivateRay(Message) (.HitActor (Collision|BreakHitResult _outhit)))
      (for _index (range 0 4)
        (Rendering|Debug|DrawDebugLine (- _returnvalue (Math|Vector|MakeVector 0.0 0.0 (* _index 5e+01))) (- (.Location (Collision|BreakHitResult _outhit)) (Math|Vector|MakeVector 0.0 0.0 (* _index 5e+01))) "(R=0.100626,G=1.000000,B=0.000000,A=1.000000)" 1.0 5.0)))))

(event Custom|Rotate
  (bind _rotations (Variables|Default|GetRotations))
  (bind _returnvalue (Utilities|Array|Length _rotations))
  (if (> _returnvalue 0)
    (bind _result (Math|Integer|IncrementInt (Variables|Default|GetIndex))
      (:%20%20
        (Variables|Default|SetIndex (Math|Integer|SelectInt 0 _result (== _result _returnvalue)))
        (Transformation|SetActorRotation (Math|Rotator|MakeRotator 0.0 0.0 (Utilities|Array|Get(acopy) (Variables|Default|GetRotations) (Variables|Default|GetIndex))))))))

(event EventBeginPlay
  (bind _emitter (Variables|Default|GetEmitter))
  (bind _index_default (Variables|Default|GetIndex_Default))
  (Transformation|SetActorRotation (Math|Rotator|MakeRotator 0.0 0.0 (Utilities|Array|Get(acopy) (Variables|Default|GetRotations) _index_default)))
  (Variables|Default|SetIndex _index_default)
  (Rendering|Material|SetMaterial (Variables|Default|GetCylinder) 0 (select (Variables|Default|GetBlocker) "/Game/Dive/Puzzle/M_Red.M_Red" (select _emitter "/Game/Dive/Puzzle/M_Green.M_Green" "/Game/Dive/Puzzle/M_Blue.M_Blue")))
  (if _emitter
    (Utilities|Time|SetTimerbyEvent (delegate Custom|SendRay) 1.0 true)))

(event Collision|EventActorBeginOverlap
  (params (OtherActor :type Actor%20Object%20Reference)))

(event EventTick
  (params (DeltaSeconds :type Float%20%28single-precision%29)))

(event EventMouseUse
  (bind _rotations (Variables|Default|GetRotations))
  (bind _returnvalue (Utilities|Array|Length _rotations))
  (if (> _returnvalue 0)
    (bind _result (Math|Integer|IncrementInt (Variables|Default|GetIndex))
      (:%20%20
        (Variables|Default|SetIndex (Math|Integer|SelectInt 0 _result (== _result _returnvalue)))
        (Transformation|SetActorRotation (Math|Rotator|MakeRotator 0.0 0.0 (Utilities|Array|Get(acopy) (Variables|Default|GetRotations) (Variables|Default|GetIndex))))))))

(event EventActivateRay
  (bind _arrow (Variables|Default|GetArrow))
  (bind _returnvalue (Transformation|GetWorldLocation _arrow))
  (if (not (Variables|Default|GetEmitter))
    (bind _outhit (Collision|LineTraceByChannel _returnvalue (+ _returnvalue (* (Math|Vector|GetForwardVector _arrow) 3e+04)) "TraceTypeQuery1" false 0 "None" true "(R=0.000000,G=0.954989,B=1.000000,A=1.000000)" "(R=1.000000,G=0.000000,B=0.972589,A=1.000000)" 1.0))
    (if (Utilities|DoesObjectImplementInterface (.HitActor (Collision|BreakHitResult _outhit)) "/Game/Dive/Puzzle/BPI_Dante.BPI_Dante_C")
      (if (not (Variables|Default|GetBlocker))
        (Class|BPIDante|ActivateRay(Message) (.HitActor (Collision|BreakHitResult _outhit)))
        (for _index (range 0 4)
          (Rendering|Debug|DrawDebugLine (- _returnvalue (Math|Vector|MakeVector 0.0 0.0 (* _index 5e+01))) (- (.Location (Collision|BreakHitResult _outhit)) (Math|Vector|MakeVector 0.0 0.0 (* _index 5e+01))) "(R=0.100626,G=1.000000,B=0.000000,A=1.000000)" 1.0 5.0))))))

(fn ConstructionScript)
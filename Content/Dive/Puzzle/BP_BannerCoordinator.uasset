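; BP_BannerCoordinator is a key-driven helper for recording banner puzzle states across all BP_Banner actors in the level.
; F10 rebuilds its stored list of banners and prints the count.
; F11 copies each listed banner's current Index into IndexDefault, and F12 copies it into IndexCorrect, capturing the start and solution states from the current arrangement.
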(event Input|KeyboardEvents|F11
  (params (Key :type Key%20Structure))
  (:Pressed
    (for _array_element (Variables|Default|GetNewVar)
      (Variables|/Game/Dive/Puzzle/BP_Banner.BP_Banner_C|SetIndex_Default _array_element (Variables|/Game/Dive/Puzzle/BP_Banner.BP_Banner_C|GetIndex _array_element)))))

(event Input|KeyboardEvents|F10
  (params (Key :type Key%20Structure))
  (bind _newvar (Variables|Default|GetNewVar))
  (:Pressed
    (Utilities|Array|Clear (Variables|Default|GetNewVar))
    (bind _outactors (Actor|GetAllActorsOfClass "/Game/Dive/Puzzle/BP_Banner.BP_Banner_C"))
    (for _array_element _outactors
      (Utilities|Array|AddUnique _newvar _array_element))
    (Development|PrintString (Utilities|String|ToString(Integer) (Utilities|Array|Length _newvar)))))

(event Input|KeyboardEvents|F12
  (params (Key :type Key%20Structure))
  (:Pressed
    (for _array_element (Variables|Default|GetNewVar)
      (Variables|/Game/Dive/Puzzle/BP_Banner.BP_Banner_C|SetIndex_Correct _array_element (Variables|/Game/Dive/Puzzle/BP_Banner.BP_Banner_C|GetIndex _array_element)))))

(fn ConstructionScript)
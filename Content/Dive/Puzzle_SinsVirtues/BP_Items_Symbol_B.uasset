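; BP_Items_Symbol_B is a collectible symbol item for the Sins and Virtues puzzle, picked up by using it with the mouse.
; MouseUse casts the player pawn to BP_FirstPersonCharacter, changes its state and adds the item to its HUD along with the symbol index and Sin value.
; The actor then destroys itself, and it has no other active logic.
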(event EventBeginPlay
  (|CallParentFunction) ; This node is disabled and will not be called.\nDrag off pins to build functionality.
)

(event Collision|EventActorBeginOverlap
  (params (OtherActor :type Actor%20Object%20Reference))
  (|CallParentFunction OtherActor) ; This node is disabled and will not be called.\nDrag off pins to build functionality.
)

(event EventTick
  (params (DeltaSeconds :type Float%20%28single-precision%29))
  (|CallParentFunction DeltaSeconds) ; This node is disabled and will not be called.\nDrag off pins to build functionality.
)

(event EventMouseUse
  (params (bClockwise :type Boolean))
  (bind _asbp_first_person_character (Utilities|Casting|CastToBP_FirstPersonCharacter (Game|Player|GetPlayerPawn 0)))
  (Default|ChangeState _asbp_first_person_character "NewEnumerator0")
  (Default|AddItem (Variables|/Game/FirstPerson/Blueprints/BP_FirstPersonCharacter.BP_FirstPersonCharacter_C|GetHUD _asbp_first_person_character) (Variables|Default|GetItem) (Variables|Default|GetIndex) (Variables|Default|GetSin))
  (Actor|DestroyActor))

(fn ConstructionScript
  (|CallParentFunction))
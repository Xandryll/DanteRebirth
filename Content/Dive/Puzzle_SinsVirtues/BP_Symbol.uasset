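; BP_Symbol is a symbol actor for the Sins and Virtues puzzle that displays either a sin or a virtue.
; SetSymbol stores the Sin flag and uses it to shift and flip the SymPivot.
; It creates a dynamic MI_Symbol material on the mesh and sets text, both looked up by Index.
; The color lookup is crossed: sins take ColorVirtues and virtues take ColorSins, while text uses the matching array.
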(event Custom|SetSymbol
  (params (Sin? :type Boolean))
  (bind _sm (Variables|Default|GetSM))
  (bind _index (Variables|Default|GetIndex))
  (Variables|Default|SetbSin Sin?)
  (Transformation|SetRelativeLocationAndRotation (Variables|Default|GetSymPivot) (Math|Vector|MakeVector 0.0 (Math|Float|SelectFloat -1.5e+02 -148.0 Sin?) 0.0) (Math|Rotator|MakeRotator 0.0 0.0 (Math|Float|SelectFloat 0.0 1.8e+02 Sin?)) false false)
  (bind _returnvalue (Rendering|Material|CreateDynamicMaterialInstance _sm 0 "/Game/Dive/Puzzle_SinsVirtues/MI_Symbol.MI_Symbol" "None" :!class /Script/Engine.PrimitiveComponent))
  (Rendering|Material|SetVectorParameterValue _returnvalue "Color" (Math|Conversions|ToLinearColor(Color) (Utilities|Array|Get(acopy) (select (Variables|Default|GetbSin) (Variables|Default|GetColorVirtues) (Variables|Default|GetColorSins)) _index)) :!class /Script/Engine.MaterialInstanceDynamic)
  (Rendering|Material|SetMaterial _sm 0 _returnvalue)
  (Rendering|Components|TextRender|SetText (Variables|Default|GetTXT) (Utilities|Array|Get(acopy) (select (Variables|Default|GetbSin) (Variables|Default|GetSins) (Variables|Default|GetVirtues)) _index)))

(event EventBeginPlay)

(fn ConstructionScript)
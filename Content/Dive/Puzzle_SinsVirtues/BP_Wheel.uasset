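; Sins and virtues wheel puzzle that spawns seven sin symbols, seven virtue symbols and eight position swappers at 45-degree steps.
; MouseUse temporarily attaches symbols with non-zero pivot yaw to the wheel mesh and turns them one position.
; SwapSymbols flips the pair at a position 180 degrees.
; After each turn, CheckSolution compares each symbol's index to its position, turning the wheel green and locking input when all match.
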(event Custom|SwapSymbols
  (params (Position :type Integer))
  (bind _as_bp_symbol_to_swap (Variables|Default|GetAs%20BP%20Symbol%20to%20Swap))
  (bind _output (Utilities|Array|Get(acopy) _as_bp_symbol_to_swap 1))
  (bind _output_2 (Utilities|Array|Get(acopy) _as_bp_symbol_to_swap))
  (bind _sympivot (Variables|/Game/Dive/Puzzle_SinsVirtues/BP_Symbol.BP_Symbol_C|GetSymPivot _output))
  (bind _sympivot_2 (Variables|/Game/Dive/Puzzle_SinsVirtues/BP_Symbol.BP_Symbol_C|GetSymPivot _output_2))
  (if (not (Variables|Default|GetbMoving))
    (Variables|Default|SetbMoving true)
    (Utilities|Array|Clear (Variables|Default|GetAs%20BP%20Symbol%20to%20Swap))
    (for _array_element (Variables|Default|GetAs%20BP%20Symbol%20All)
      (if (== Position (Variables|/Game/Dive/Puzzle_SinsVirtues/BP_Symbol.BP_Symbol_C|GetPositionIndex _array_element))
        (Utilities|Array|AddUnique (Variables|Default|GetAs%20BP%20Symbol%20to%20Swap) _array_element)))
    (Variables|Default|SetSymARot (.yaw (Variables|/Script/Engine.SceneComponent|GetRelativeRotation _sympivot_2)))
    (Variables|Default|SetSymBRot (.yaw (Variables|/Script/Engine.SceneComponent|GetRelativeRotation _sympivot)))
    (bind _newtrack_0 (Timeline|Timeline_0 PlayFromStart)
      (:Update
        (Transformation|SetRelativeRotation _sympivot_2 (Math|Rotator|MakeRotator 0.0 0.0 (Math|Float|SelectFloat 0.0 (+ (Math|Float|Lerp 0.0 1.8e+02 _newtrack_0) (Variables|Default|GetSymARot)) (== (+ (Math|Float|Lerp 0.0 1.8e+02 _newtrack_0) (Variables|Default|GetSymARot)) 3.6e+02))) false false)
        (Transformation|SetRelativeRotation _sympivot (Math|Rotator|MakeRotator 0.0 0.0 (Math|Float|SelectFloat 0.0 (+ (Math|Float|Lerp 0.0 1.8e+02 _newtrack_0) (Variables|Default|GetSymBRot)) (== (+ (Math|Float|Lerp 0.0 1.8e+02 _newtrack_0) (Variables|Default|GetSymBRot)) 3.6e+02))) false false))
      (:Finished
        (Variables|Default|SetbMoving false)))))

(event Custom|CheckSolution
  (bind _array_element (Utilities|Array|ForEachLoopwithBreak (Variables|Default|GetAs%20BP%20Symbol%20All) :!label _label)
    (:LoopBody
      (Development|PrintString (Utilities|String|Append (Utilities|GetDisplayName _array_element) (Utilities|String|ToString(Boolean) (== (Variables|/Game/Dive/Puzzle_SinsVirtues/BP_Symbol.BP_Symbol_C|GetIndex _array_element) (Variables|/Game/Dive/Puzzle_SinsVirtues/BP_Symbol.BP_Symbol_C|GetPositionIndex _array_element))) " " (Utilities|String|ToString(Integer) (Variables|/Game/Dive/Puzzle_SinsVirtues/BP_Symbol.BP_Symbol_C|GetIndex _array_element)) " - " (Utilities|String|ToString(Integer) (Variables|/Game/Dive/Puzzle_SinsVirtues/BP_Symbol.BP_Symbol_C|GetPositionIndex _array_element))))
      (bind _output_get (Variables|Default|SetbSolved (== (Variables|/Game/Dive/Puzzle_SinsVirtues/BP_Symbol.BP_Symbol_C|GetIndex _array_element) (Variables|/Game/Dive/Puzzle_SinsVirtues/BP_Symbol.BP_Symbol_C|GetPositionIndex _array_element))))
      (if (not _output_get)
        (goto _label Break)))
    (:Completed
      (if (Variables|Default|GetbSolved)
        (Rendering|Material|SetMaterial (Variables|Default|GetSM) 0 "/Game/Dive/Puzzle_CrowdsLabyrint/M_Green.M_Green")
        (Variables|Default|SetbMoving true)))))

(event EventBeginPlay
  (Utilities|Array|Clear (Variables|Default|GetAs%20BP%20Symbol%20InternalRing))
  (Utilities|FlowControl|Sequence
    (:then_0
      (Utilities|Array|Clear (Variables|Default|GetAs%20BP%20Symbol%20Sins))
      (for _index (range 1 7)
        (bind _returnvalue (AddComponent|AddChildActorComponent false))
        (Transformation|SetRelativeRotation _returnvalue (Math|Rotator|MakeRotator 0.0 0.0 (+ (Math|Conversions|ToFloat(Integer) (* _index -45)) 1.8e+02)) false false)
        (bind _asbp_symbol (Utilities|Casting|CastToBP_Symbol (Variables|/Script/Engine.ChildActorComponent|GetChildActor _returnvalue)))
        (Utilities|Array|AddUnique (Variables|Default|GetAs%20BP%20Symbol%20Sins) _asbp_symbol)
        (Utilities|Array|AddUnique (Variables|Default|GetAs%20BP%20Symbol%20All) _asbp_symbol)
        (Variables|/Game/Dive/Puzzle_SinsVirtues/BP_Symbol.BP_Symbol_C|SetIndex _asbp_symbol (- _index 1))
        (Variables|/Game/Dive/Puzzle_SinsVirtues/BP_Symbol.BP_Symbol_C|SetPositionIndex _asbp_symbol (- _index 1))
        (Default|SetSymbol _asbp_symbol true)))
    (:then_1
      (Utilities|Array|Clear (Variables|Default|GetAs%20BP%20Symbol%20Virtues))
      (for _index_2 (range 1 7)
        (bind _returnvalue_2 (AddComponent|AddChildActorComponent false))
        (Transformation|SetRelativeRotation _returnvalue_2 (Math|Rotator|MakeRotator 0.0 0.0 (+ (Math|Conversions|ToFloat(Integer) (* _index_2 -45)) 1.8e+02)) false false)
        (bind _asbp_symbol_2 (Utilities|Casting|CastToBP_Symbol (Variables|/Script/Engine.ChildActorComponent|GetChildActor _returnvalue_2)))
        (Utilities|Array|AddUnique (Variables|Default|GetAs%20BP%20Symbol%20Virtues) _asbp_symbol_2)
        (Utilities|Array|AddUnique (Variables|Default|GetAs%20BP%20Symbol%20All) _asbp_symbol_2)
        (Variables|/Game/Dive/Puzzle_SinsVirtues/BP_Symbol.BP_Symbol_C|SetIndex _asbp_symbol_2 (- _index_2 1))
        (Variables|/Game/Dive/Puzzle_SinsVirtues/BP_Symbol.BP_Symbol_C|SetPositionIndex _asbp_symbol_2 (- _index_2 1))
        (Default|SetSymbol _asbp_symbol_2 false)))
    (:then_2
      (for _index_3 (range 0 7)
        (bind _returnvalue_3 (AddComponent|AddChildActorComponent false))
        (Transformation|SetRelativeRotation _returnvalue_3 (Math|Rotator|MakeRotator 0.0 0.0 (+ (Math|Conversions|ToFloat(Integer) (* _index_3 -45)) 1.8e+02)) false false)
        (bind _asbp_symbol_swapper (Utilities|Casting|CastToBP_SymbolSwapper (Variables|/Script/Engine.ChildActorComponent|GetChildActor _returnvalue_3)))
        (Variables|/Game/Dive/Puzzle_SinsVirtues/BP_SymbolSwapper.BP_SymbolSwapper_C|SetPositionIndex _asbp_symbol_swapper _index_3)))))

(event EventMouseUse
  (bind _sm (Variables|Default|GetSM))
  (bind _as_bp_symbol_internalring (Variables|Default|GetAs%20BP%20Symbol%20InternalRing))
  (if (not (Variables|Default|GetbMoving))
    (for _array_element (Variables|Default|GetAs%20BP%20Symbol%20All)
      (if (not (== (Math|Float|Truncate (.yaw (Variables|/Script/Engine.SceneComponent|GetRelativeRotation (Variables|/Game/Dive/Puzzle_SinsVirtues/BP_Symbol.BP_Symbol_C|GetSymPivot _array_element)))) 0.0))
        (Development|PrintString (Utilities|String|Append "OBJ: " (Utilities|GetDisplayName _array_element) " - Rot: " (Utilities|String|ToString(Float) (.yaw (Variables|/Script/Engine.SceneComponent|GetRelativeRotation (Variables|/Game/Dive/Puzzle_SinsVirtues/BP_Symbol.BP_Symbol_C|GetSymPivot _array_element))))))
        (Utilities|Array|AddUnique (Variables|Default|GetAs%20BP%20Symbol%20InternalRing) _array_element)
        (Variables|Default|SetbMoving true)
        (for _array_element_2 (Variables|Default|GetAs%20BP%20Symbol%20InternalRing)
          (Transformation|AttachComponentToComponent _array_element_2 (Variables|Default|GetSM) "None" "KeepWorld" "KeepWorld" "KeepWorld" true))
        (Variables|Default|SetPrevRot (.yaw (Variables|/Script/Engine.SceneComponent|GetRelativeRotation _sm)))
        (bind _newtrack_0 (Timeline|Timeline PlayFromStart)
          (:Update
            (Transformation|SetRelativeRotation _sm (Math|Rotator|MakeRotator 0.0 0.0 (+ (* _newtrack_0 -45.0) (Variables|Default|GetPrevRot))) false false))
          (:Finished
            (for _array_element_3 _as_bp_symbol_internalring
              (bind _result (Math|Integer|IncrementInt (Variables|/Game/Dive/Puzzle_SinsVirtues/BP_Symbol.BP_Symbol_C|GetPositionIndex _array_element_3))
                (:%20%20
                  (bind _output_get (Variables|/Game/Dive/Puzzle_SinsVirtues/BP_Symbol.BP_Symbol_C|SetPositionIndex _array_element_3 (Math|Integer|SelectInt 0 (Variables|/Game/Dive/Puzzle_SinsVirtues/BP_Symbol.BP_Symbol_C|GetPositionIndex _array_element_3) (> _result 7))))
                  (Transformation|AttachComponentToComponent _array_element_3 (Variables|Default|GetDefaultSceneRoot) "None" "KeepWorld" "KeepWorld" "KeepWorld" true)
                  (Development|PrintString (Utilities|String|Append (Utilities|GetDisplayName _array_element_3) " - " (Utilities|String|ToString(Integer) _output_get))))))
            (Utilities|Array|Clear _as_bp_symbol_internalring)
            (Variables|Default|SetbMoving false)
            (CallFunction|CheckSolution)))))))

(fn ConstructionScript)